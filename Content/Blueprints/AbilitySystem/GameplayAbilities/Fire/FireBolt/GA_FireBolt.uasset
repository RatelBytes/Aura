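; Fire Bolt gameplay ability that casts a projectile toward the location under the mouse cursor.
; A target-data task supplies the hit location, which turns the caster through AuraCombatInterface before the cast montage plays.
; A gameplay event sent by the montage's AN_MontageEvent notify triggers SpawnProjectile, syncing the spawn to the animation.
; The ability ends after a short delay following the spawn, with no handling for montage interruption.
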(event Ability|EventActivateAbility
  (bind _datahandle (|AuraTargetDataUnderMouse)
    (:ValidDataDelegate
      (Variables|Default|SetProjectileTargetLocation (.Location (Collision|BreakHitResult (Ability|TargetData|GetHitResultfromTargetData _datahandle))))
      (bind _asaura_combat_interface (Utilities|Casting|CastToAuraCombatInterface (Ability|GetAvatarActorfromActorInfo)))
      (Class|AuraCombatInterface|UpdateFacingTarget _asaura_combat_interface (Variables|Default|GetProjectileTargetLocation))
      (|PlayMontageandWaitProxy "None" "/Game/Assets/Characters/Aura/Animations/Abilities/AM_Cast_FireBolt.AM_Cast_FireBolt" 1.0 "None" true 1.0 0.0
        (:then
          ;[1 1 1] We send a gameplay event with Event Tag thanks to AN_MontageEvent. And when it is received, we execute next node
          (Ability|Tasks|WaitGameplayEvent "(TagName=\"Event.Montage.FireBolt\")" 0
            (:EventReceived
              (Class|AuraProjectileSpell|SpawnProjectile (Variables|Default|GetProjectileTargetLocation))
              (Utilities|FlowControl|Delay 0.5)
              (Ability|EndAbility))))))))

(event Ability|EventOnEndAbility
  (params (bWasCancelled :type Boolean)))